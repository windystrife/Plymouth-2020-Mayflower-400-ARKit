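; AR player pawn that places a pre-existing portal pair on a detected plane with a single successful touch, once MainWidget allows it.
; Tick gates placement on Normal tracking, downgraded on Android until planes are found.
; Touch hit-tests via ARCore or ARKit, then aligns portals and blockers to face the camera.
; Only the iOS path sets 360 materials and info-panel visibility from widget choices; portal teleport logic is unwired.
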(fn `CachePlatform`
  ;[1 1 1] Cache platform that we're running on for switching on platform-specific functionality
  (bind _returnvalue (`GameplayStatics.GetPlatformName`))
  (bind _output_get (set `self.bIsAndroid` (== _returnvalue "Android")))
  (`KismetSystemLibrary.PrintString` _returnvalue)
  (`KismetSystemLibrary.PrintString` (`KismetStringLibrary.Conv_BoolToString` _output_get)))

(fn `DetermineTrackingQuality`
  (returns (Tracking :type "EARTrackingQuality Enum"))
  (locals (TrackingQuality :type "EARTrackingQuality Enum"))
  (bind _returnvalue (`ARBlueprintFunctionLibrary.GetTrackingQuality`))
  ;[1 1 1] If we haven't found any planes yet, downgrade the tracking quality by 1 notch.
  (bind _output_get (set `local.TrackingQuality` _returnvalue))
  (bind _returnvalue_2 (select `bool` (>= (`self.numPlanesDetected`) 1) :`false` (select `EARTrackingQuality` _output_get :`NotAvailable` "NotAvailable" :`Limited` "Limited" :`Normal` "Limited" :!type "EARTrackingQuality Enum") :`true` _output_get))
  (set `self.TrackingQualityPublic` _returnvalue_2)
  (return _returnvalue_2))

(fn `DisplayDebugTrackingInfo`
  ;[1 1 1] Display Debug Tracking Info
  (`KismetSystemLibrary.PrintString` (`KismetStringLibrary.Conv_TransformToString` (`SceneComponent.K2_GetComponentToWorld` (`PlayerCameraManager.TransformComponent` (`GameplayStatics.GetPlayerCameraManager` 0)))) true false (struct :`R` 0.081168 :`G` 1.0 :`B` 0.218801 :`A` 1.0) 0.0)
  (bind _tracking (`self.DetermineTrackingQuality`))
  (`KismetSystemLibrary.PrintString` (`KismetStringLibrary.Concat_StrStr` "[ " (`|GetEnumeratorNameAsString` _tracking) " ]") true false (select `EARTrackingQuality` _tracking :`NotAvailable` (struct :`R` 1.0 :`B` 0.158961 :`A` 1.0) :`Limited` (struct :`R` 1.0 :`G` 0.226966 :`A` 1.0) :`Normal` (struct :`R` 0.283149 :`G` 1.0 :`A` 1.0) :!type "LinearColor Structure") 0.0))

(fn `DoHitTestForARCORE`
  (params (Player :type "PlayerController Object Reference") (InputPin :type "Vector2D Structure"))
  (returns (Success :type Boolean) (SpawnTransform :type "Transform Structure") (Plane :type "GoogleARCorePlane Object Reference"))
  (bind (_worldposition _worlddirection) (`GameplayStatics.DeprojectScreenToWorld` Player InputPin))
  (bind (_impactpoint _impactnormal _outplaneobject _returnvalue) (`GoogleARCoreSessionFunctionLibrary.LineTraceSingleOnPlanes` _worldposition (+ _worldposition (* _worlddirection 10000.0))))
  (if _returnvalue
    (`KismetSystemLibrary.PrintString` (`KismetStringLibrary.Concat_StrStr` "HIT from :  " (`KismetStringLibrary.Conv_Vector2dToString` InputPin)) true true (struct :`R` 0.7074 :`G` 1.0 :`A` 1.0))
    (bind _returnvalue_2 (`KismetMathLibrary.MakeTransform` _impactpoint))
    (`KismetSystemLibrary.PrintString` (`KismetStringLibrary.Conv_TransformToString` _returnvalue_2) true true (struct :`R` 1.0 :`G` 0.96541 :`A` 1.0))
    (return true (`KismetMathLibrary.MakeTransform` (.location _returnvalue_2) (`KismetMathLibrary.MakeRotator` (.roll (`KismetMathLibrary.FindLookAtRotation` _impactpoint (+ _impactpoint (`KismetMathLibrary.Normal` (* _worlddirection (1.0 1.0 0.0)))))) (.pitch (`KismetMathLibrary.FindLookAtRotation` _impactpoint (+ _impactpoint (`KismetMathLibrary.Normal` (* _worlddirection (1.0 1.0 0.0)))))) (+ (.yaw (`KismetMathLibrary.FindLookAtRotation` _impactpoint (+ _impactpoint (`KismetMathLibrary.Normal` (* _worlddirection (1.0 1.0 0.0)))))) 180.0)) (.scale _returnvalue_2)) _outplaneobject)
    (else
      (return false (struct) null))))

(fn `DoHitTestForARKIT`
  (params (InputPin :type "Vector2D Structure") (PlayerController :type "PlayerController Object Reference"))
  (returns (Success :type Boolean) (SpawnTransform :type "Transform Structure"))
  (bind (_outresults _returnvalue) (`AppleARKitBlueprintLibrary.HitTestAtScreenPosition_TrackingSpace` InputPin "ExistingPlane"))
  (if _returnvalue
    (bind (_type _distance _transform) (break `AppleARKitHitTestResult` (`|GetArrayItem` _outresults)))
    (`KismetSystemLibrary.PrintString` (`KismetStringLibrary.Concat_StrStr` "HIT from :  " (`KismetStringLibrary.Conv_Vector2dToString` InputPin) " Distance : " (`KismetStringLibrary.Conv_DoubleToString` _distance)) true true (struct :`R` 0.7074 :`G` 1.0 :`A` 1.0))
    (`KismetSystemLibrary.PrintString` (`KismetStringLibrary.Conv_TransformToString` _transform) true true (struct :`R` 1.0 :`G` 0.96541 :`A` 1.0))
    (bind _location (.location _transform))
    (return true (`KismetMathLibrary.MakeTransform` _location (`KismetMathLibrary.MakeRotator` (.roll (`KismetMathLibrary.FindLookAtRotation` _location (+ _location (`KismetMathLibrary.Normal` (* (`.WorldDirection` (`GameplayStatics.DeprojectScreenToWorld` PlayerController InputPin)) (1.0 1.0 0.0)))))) (.pitch (`KismetMathLibrary.FindLookAtRotation` _location (+ _location (`KismetMathLibrary.Normal` (* (`.WorldDirection` (`GameplayStatics.DeprojectScreenToWorld` PlayerController InputPin)) (1.0 1.0 0.0)))))) (+ (.yaw (`KismetMathLibrary.FindLookAtRotation` _location (+ _location (`KismetMathLibrary.Normal` (* (`.WorldDirection` (`GameplayStatics.DeprojectScreenToWorld` PlayerController InputPin)) (1.0 1.0 0.0)))))) 180.0)) (.scale _transform)))
    (else
      (return false))))

(fn `FindPlanesForARCORE`
  (bind _outarcoreplanelist (`GoogleARCoreFrameFunctionLibrary.GetAllPlanes`))
  (bind _returnvalue (`KismetArrayLibrary.Array_Length` _outarcoreplanelist))
  (`KismetSystemLibrary.PrintString` (`KismetStringLibrary.Conv_IntToString` _returnvalue) true false (struct :`G` 0.66 :`B` 1.0 :`A` 1.0) 0.0)
  (set `self.numPlanesDetected` _returnvalue))

(fn `UserConstructionScript`)